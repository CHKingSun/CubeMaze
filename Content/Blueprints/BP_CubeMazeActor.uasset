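; Cube-shaped maze actor built from six child-actor maze faces: left, right, front, back, top and bottom.
; The construction script assigns MazeClass to every face, then gives each BP_MazeActor child its own hard-coded floor color through SetMazeFloorColor.
; It finishes by calling GenerateCubeMaze, whose body is not in this graph.
; The event graph holds no runtime logic.
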(event `self.ReceiveBeginPlay`)

(fn `SetMazeFloorColor`
  (params (Child :type "ChildActorComponent Object Reference") (Color :type "LinearColor Structure"))
  (bind _asbp_maze_actor (cast `/Game/Blueprints/BP_MazeActor` (`ChildActorComponent.ChildActor` Child)))
  (`/Game/Blueprints/BP_MazeActor.SetFloorColor` _asbp_maze_actor Color))

(fn `UserConstructionScript`
  (locals (MazeClass :type "Actor Class Reference" :default "BlueprintGeneratedClass'/Game/Blueprints/BP_MazeActor.BP_MazeActor_C'"))
  (bind _mazeleft (`self.MazeLeft`))
  (`ChildActorComponent.SetChildActorClass` _mazeleft (`local.MazeClass`))
  (`ChildActorComponent.SetChildActorClass` (`self.MazeFront`) (`local.MazeClass`))
  (`ChildActorComponent.SetChildActorClass` (`self.MazeBack`) (`local.MazeClass`))
  (`ChildActorComponent.SetChildActorClass` (`self.MazeTop`) (`local.MazeClass`))
  (`ChildActorComponent.SetChildActorClass` (`self.MazeBottom`) (`local.MazeClass`))
  (`ChildActorComponent.SetChildActorClass` (`self.MazeRight`) (`local.MazeClass`))
  (`|ExecutionSequence`
    (:`then_0`
      (`self.SetMazeFloorColor` _mazeleft (struct :`R` 0.815686 :`G` 0.062745 :`B` 0.298039 :`A` 1.0)))
    (:`then_1`
      (`self.SetMazeFloorColor` (`self.MazeFront`) (struct :`R` 0.180392 :`G` 0.360784 :`B` 0.431373 :`A` 1.0)))
    (:`then_2`
      (`self.SetMazeFloorColor` (`self.MazeBack`) (struct :`R` 0.176471 :`G` 0.427451 :`B` 0.294118 :`A` 1.0)))
    (:`then_3`
      (`self.SetMazeFloorColor` (`self.MazeTop`) (struct :`R` 0.988235 :`G` 0.980392 :`B` 0.94902 :`A` 1.0)))
    (:`then_4`
      (`self.SetMazeFloorColor` (`self.MazeBottom`) (struct :`R` 1.0 :`G` 0.657895 :`A` 1.0)))
    (:`then_5`
      (`self.SetMazeFloorColor` (`self.MazeRight`) (struct :`R` 0.651042 :`G` 0.268778 :`A` 1.0)))
    (:`then_6`
      (`self.GenerateCubeMaze` true))))